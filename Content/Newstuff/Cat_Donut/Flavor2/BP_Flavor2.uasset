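; BP_Flavor2 is an actor in the Cat_Donut folder that currently only caches a reference to the first-person player character on BeginPlay.
; Its Tick event is empty, so the actor does nothing per frame.
; Disconnected logic would turn it away from the player when recently rendered and toward the player otherwise, but that branch never runs.
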(event `self.ReceiveBeginPlay`
  (bind _returnvalue (`GameplayStatics.GetActorOfClass` "/Game/FirstPerson/Blueprints/BP_FirstPersonCharacter.BP_FirstPersonCharacter_C"))
  (set `self.player` _returnvalue))

(event `self.ReceiveTick`
  (params (DeltaSeconds :type "Float (single-precision)")))

(fn `UserConstructionScript`)