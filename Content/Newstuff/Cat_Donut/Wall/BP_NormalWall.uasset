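; BP_NormalWall is a breakable wall that shatters when hit by the BP_FirstPersonProjectile_2 projectile.
; Every tick it checks the actors overlapping its Box1 volume by comparing class display name strings rather than casting.
; On a match, a DoOnce spawns a slightly upscaled BP_ShatterWallLong at the wall's transform, destroys the wall and plays a 2D concrete break sound.
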(event `self.ReceiveTick`
  (params (DeltaSeconds :type "Float (single-precision)"))
  (for _array_element (`PrimitiveComponent.GetOverlappingActors` (`self.Box1`) "/Script/Engine.Actor")
    (if (`KismetStringLibrary.EqualEqual_StrStr` (`KismetSystemLibrary.GetClassDisplayName` (`GameplayStatics.GetObjectClass` _array_element)) "BP_FirstPersonProjectile_2_C")
      (`/Engine/EditorBlueprintResources/StandardMacros.DoOnce` false
        (:`Completed`
          (`|SpawnActorFromClass` "/Game/Newstuff/Cat_Donut/Wall/BP_ShatterWallLong.BP_ShatterWallLong_C" (`KismetMathLibrary.MakeTransform` (.location (`self.GetTransform`)) (.rotation (`self.GetTransform`)) (* (.scale (`self.GetTransform`)) 1.05)) "Undefined" "OverrideRootScale" null null)
          (`self.K2_DestroyActor`)
          (`GameplayStatics.PlaySound2D` "/Game/Newstuff/Cat_Donut/Flavor2/Concrete_Break_Sound_Effect.Concrete_Break_Sound_Effect" 1.0 1.0 0.0 null null))))))

(fn `UserConstructionScript`)