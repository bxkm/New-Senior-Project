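; BP_CatDonut is an interactable cat donut actor that shows a widget while something overlaps its box and distorts its scale when used.
; Each Interact toggles a particle system, adds a random offset to scale, and randomly switches a chaos state on or off.
; During chaos, Tick subtracts random scale offsets for a fixed number of frames, then holds the size saved when chaos began.
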(event `self.Box.OnComponentBeginOverlap`
  (params (OverlappedComponent :type "PrimitiveComponent Object Reference") (OtherActor :type "Actor Object Reference") (OtherComp :type "PrimitiveComponent Object Reference") (OtherBodyIndex :type Integer) (bFromSweep :type Boolean) (SweepResult :type "HitResult Structure (by ref)"))
  (`SceneComponent.SetHiddenInGame` (`self.Widget`) false false))

(event `self.Box.OnComponentEndOverlap`
  (params (OverlappedComponent :type "PrimitiveComponent Object Reference") (OtherActor :type "Actor Object Reference") (OtherComp :type "PrimitiveComponent Object Reference") (OtherBodyIndex :type Integer))
  (`SceneComponent.SetHiddenInGame` (`self.Widget`) true false))

(event `/Game/FirstPerson/Blueprints/InteractInterface.Interact`
  (bind _particlesystem (`self.ParticleSystem`))
  (`/Engine/EditorBlueprintResources/StandardMacros.FlipFlop`
    (:`A`
      (`SceneComponent.SetHiddenInGame` _particlesystem false false))
    (:`B`
      (`SceneComponent.SetHiddenInGame` _particlesystem true false)))
  (`self.SetActorScale3D` (+ (`self.GetActorScale3D`) (`KismetMathLibrary.MakeVector` (`KismetMathLibrary.RandomFloatInRange` -1.0 2.5) (`KismetMathLibrary.RandomFloatInRange` -1.0 3.0) (`KismetMathLibrary.RandomFloatInRange` -1.0 3.0))))
  (`/Engine/EditorBlueprintResources/StandardMacros.CompareInt` (`KismetMathLibrary.RandomIntegerInRange` 0 3)
    (:`>`
      (set `self.Cat Chaos` false :!label _label))
    (:`==`
      (set `self.Cat Chaos` true)
      (set `self.CatOriginalSize` (`self.GetActorScale3D`))
      (set `self.counter` 0))
    (:`<`
      (goto _label))))

(event `self.ReceiveTick`
  (params (DeltaSeconds :type "Float (single-precision)"))
  (if (`self.Cat Chaos`)
    (bind _output_get (set `self.counter` (+ 1 (`self.counter`))))
    (`/Engine/EditorBlueprintResources/StandardMacros.CompareInt` _output_get 55
      (:`>`
        (`self.SetActorScale3D` (`self.CatOriginalSize`)))
      (:`<`
        (`self.SetActorScale3D` (- (`self.GetActorScale3D`) (`KismetMathLibrary.MakeVector` (`KismetMathLibrary.RandomFloatInRange` -1.0 2.5) (`KismetMathLibrary.RandomFloatInRange` -1.0 3.0) (`KismetMathLibrary.RandomFloatInRange` -1.0 3.0))))))))

(fn `UserConstructionScript`)