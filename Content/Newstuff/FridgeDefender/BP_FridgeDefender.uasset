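; Fridge defender actor that shows a widget on overlap; interacting toggles its door and, on opening, reveals mannequin arms and activates it.
; While active, Tick turns it toward the BP_Flavor2 cached at BeginPlay.
; With the player's DevMode2 on, it advances and spawns egg projectiles from its Egg socket, throttled by nested FlipFlops.
; With no BP_Flavor2 left, it targets and moves toward the player.
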(event `self.UI 'E'.OnComponentBeginOverlap`
  (params (OverlappedComponent :type "PrimitiveComponent Object Reference") (OtherActor :type "Actor Object Reference") (OtherComp :type "PrimitiveComponent Object Reference") (OtherBodyIndex :type Integer) (bFromSweep :type Boolean) (SweepResult :type "HitResult Structure (by ref)"))
  (`SceneComponent.SetHiddenInGame` (`self.Widget`) false false))

(event `self.UI 'E'.OnComponentEndOverlap`
  (params (OverlappedComponent :type "PrimitiveComponent Object Reference") (OtherActor :type "Actor Object Reference") (OtherComp :type "PrimitiveComponent Object Reference") (OtherBodyIndex :type Integer))
  (`SceneComponent.SetHiddenInGame` (`self.Widget`) true false))

(event `/Game/FirstPerson/Blueprints/InteractInterface.Interact`
  ;[1 1 1] Opening door and spawing egg once interacted
  (`/Engine/EditorBlueprintResources/StandardMacros.FlipFlop`
    (:`A`
      (bind (_direction _door_track) (`Timeline|Timeline_2` :!label _label)
        (:`Update`
          (`SceneComponent.K2_SetRelativeRotation` (`self.Fdoor`) (`KismetMathLibrary.MakeRotator` 0.0 0.0 (`KismetMathLibrary.Lerp` 0.0 -90.0 _door_track)) false false)
          (`SceneComponent.SetVisibility` (`self.SK_Mannequin_Arms`) true false)
          (set `self.ArmsScale` true))))
    (:`B`
      (goto _label :!via `Reverse`))))

(event `self.ReceiveBeginPlay`
  (bind _returnvalue (`GameplayStatics.GetActorOfClass` "/Game/Newstuff/Cat_Donut/Flavor2/BP_Flavor2.BP_Flavor2_C"))
  (set `self.TargetOrDonutBP` _returnvalue))

(event `self.ReceiveTick`
  (params (DeltaSeconds :type "Float (single-precision)"))
  (bind _returnvalue (`self.K2_GetActorLocation`))
  (bind _returnvalue_2 (`self.GetDistanceTo` (`self.TargetOrDonutBP`)))
  (bind _returnvalue_3 (+ _returnvalue (50.0 0.0 70.0)))
  (bind _returnvalue_4 (`KismetMathLibrary.FindLookAtRotation` _returnvalue_3 (`self.K2_GetActorLocation` (`self.TargetOrDonutBP`))))
  ;[1 1 1] Opening door and spawing egg once interacted
  (if (`self.ArmsScale`)
    (bind _outactors (`GameplayStatics.GetAllActorsOfClass` "/Game/Newstuff/Cat_Donut/Flavor2/BP_Flavor2.BP_Flavor2_C"))
    (`/Engine/EditorBlueprintResources/StandardMacros.CompareInt` (`KismetArrayLibrary.Array_Length` _outactors)
      (:`>`
        (`self.K2_SetActorRotation` _returnvalue_4)
        (bind _returnvalue_5 (`GameplayStatics.GetActorOfClass` "/Game/FirstPerson/Blueprints/BP_FirstPersonCharacter.BP_FirstPersonCharacter_C"))
        (if (`/Game/FirstPerson/Blueprints/BP_FirstPersonCharacter.DevMode2` _returnvalue_5)
          (`/Engine/EditorBlueprintResources/StandardMacros.CompareFloat` _returnvalue_2 1.0
            (:`>`
              (`self.K2_SetActorLocation` (+ (* (`KismetMathLibrary.GetForwardVector` _returnvalue_4) (`KismetMathLibrary.Lerp` (`KismetMathLibrary.FClamp` _returnvalue_2))) _returnvalue))
              (`/Engine/EditorBlueprintResources/StandardMacros.FlipFlop`
                (:`B`
                  (`/Engine/EditorBlueprintResources/StandardMacros.FlipFlop`
                    (:`B`
                      (`/Engine/EditorBlueprintResources/StandardMacros.FlipFlop`
                        (:`B`
                          (`/Engine/EditorBlueprintResources/StandardMacros.FlipFlop`
                            (:`B`
                              (`|SpawnActorFromClass` "/Game/FirstPerson/Blueprints/BP_FirstPersonProjectile_2.BP_FirstPersonProjectile_2_C" (`KismetMathLibrary.MakeTransform` (+ (.location (`SceneComponent.GetSocketTransform` (`self.refrigeratorbody`) "Egg" "RTS_World")) (`KismetMathLibrary.Vector_Forward`)) (struct :`Roll` 90.0) (.scale (`SceneComponent.GetSocketTransform` (`self.refrigeratorbody`) "Egg" "RTS_World"))) "Undefined" "OverrideRootScale" null null)))))))))))))
      (:`==`
        (bind _returnvalue_6 (`GameplayStatics.GetActorOfClass` "/Game/FirstPerson/Blueprints/BP_FirstPersonCharacter.BP_FirstPersonCharacter_C"))
        (set `self.TargetOrDonutBP` _returnvalue_6)
        (`self.K2_SetActorRotation` _returnvalue_4)
        (`self.K2_SetActorLocation` (+ (* (`KismetMathLibrary.GetForwardVector` _returnvalue_4) 1.0) _returnvalue_3))))))

(fn `UserConstructionScript`)