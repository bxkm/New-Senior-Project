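; BP_InfoOilBottle is an interactable oil bottle pickup tied to the player's current objective.
; A box overlap shows or hides its widget.
; Interact checks that the first-person character's current objective matches its own, then once spawns BP_HeldOilBottle attached to the GripPoint socket and destroys itself.
; It also looks up BP_InfoPan actors before destruction but leaves the result unused.
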(event `self.Box.OnComponentBeginOverlap`
  (params (OverlappedComponent :type "PrimitiveComponent Object Reference") (OtherActor :type "Actor Object Reference") (OtherComp :type "PrimitiveComponent Object Reference") (OtherBodyIndex :type Integer) (bFromSweep :type Boolean) (SweepResult :type "HitResult Structure (by ref)"))
  (`SceneComponent.SetHiddenInGame` (`self.Widget`) false false))

(event `self.Box.OnComponentEndOverlap`
  (params (OverlappedComponent :type "PrimitiveComponent Object Reference") (OtherActor :type "Actor Object Reference") (OtherComp :type "PrimitiveComponent Object Reference") (OtherBodyIndex :type Integer))
  (`SceneComponent.SetHiddenInGame` (`self.Widget`) true false))

(event `/Game/FirstPerson/Blueprints/InteractInterface.Interact`
  ;[1 1 1] Spawn Oil Bottle
  (bind _asbp_first_person_character (cast `/Game/FirstPerson/Blueprints/BP_FirstPersonCharacter` (`GameplayStatics.GetPlayerCharacter` 0))
    (:`then`
      (if (`KismetStringLibrary.EqualEqual_StrStr` (`/Game/FirstPerson/Blueprints/BP_FirstPersonCharacter.CurrentObjective` _asbp_first_person_character) (`self.Objective`))
        (`/Engine/EditorBlueprintResources/StandardMacros.DoOnce` false
          (:`Completed`
            (bind _firstpersonmesh (`/Game/FirstPerson/Blueprints/BP_FirstPersonCharacter.FirstPersonMesh` _asbp_first_person_character))
            (bind _returnvalue (`|SpawnActorFromClass` "/Game/Newstuff/KitchenAssets/Oil/BP_HeldOilBottle.BP_HeldOilBottle_C" (`SceneComponent.GetSocketTransform` _firstpersonmesh "GripPoint" "RTS_World") "Undefined" "OverrideRootScale" null null))
            (`self.K2_AttachToComponent` _returnvalue _firstpersonmesh "GripPoint" "SnapToTarget" "SnapToTarget" "SnapToTarget" true)
            (`GameplayStatics.GetAllActorsOfClass` "/Game/Newstuff/KitchenAssets/Pan/BP_InfoPan.BP_InfoPan_C")
            (`self.K2_DestroyActor`)))))
    (:`CastFailed`
      (`KismetSystemLibrary.PrintString` "no work"))))

(fn `UserConstructionScript`)