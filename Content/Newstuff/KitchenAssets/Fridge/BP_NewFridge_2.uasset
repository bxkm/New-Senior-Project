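; Interactable kitchen fridge that opens its door and gives the player an egg, gated by the character's current objective or DevMode.
; Overlap toggles a prompt widget; Interact swings the door on a timeline, then spawns BP_egg attached to the GripPoint socket.
; Taking the egg moves the custom-depth highlight from fridge to pan, and further interaction toggles the door.
; Tick holds a CatChaos scale-jitter effect, but its trigger logic is unconnected.
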(event `self.UI 'E'.OnComponentBeginOverlap`
  (params (OverlappedComponent :type "PrimitiveComponent Object Reference") (OtherActor :type "Actor Object Reference") (OtherComp :type "PrimitiveComponent Object Reference") (OtherBodyIndex :type Integer) (bFromSweep :type Boolean) (SweepResult :type "HitResult Structure (by ref)"))
  (`SceneComponent.SetHiddenInGame` (`self.Widget`) false false))

(event `self.UI 'E'.OnComponentEndOverlap`
  (params (OverlappedComponent :type "PrimitiveComponent Object Reference") (OtherActor :type "Actor Object Reference") (OtherComp :type "PrimitiveComponent Object Reference") (OtherBodyIndex :type Integer))
  (`SceneComponent.SetHiddenInGame` (`self.Widget`) true false))

(event `/Game/FirstPerson/Blueprints/InteractInterface.Interact`
  ;[1 1 1] Opening door and spawing egg once interacted
  (bind _asbp_first_person_character (cast `/Game/FirstPerson/Blueprints/BP_FirstPersonCharacter` (`GameplayStatics.GetPlayerCharacter` 0)))
  (if (or (`KismetStringLibrary.EqualEqual_StrStr` (`/Game/FirstPerson/Blueprints/BP_FirstPersonCharacter.CurrentObjective` _asbp_first_person_character) (`self.Objective`)) (`/Game/FirstPerson/Blueprints/BP_FirstPersonCharacter.DevMode` _asbp_first_person_character))
    (if (`self.IsDoorClose`)
      (`/Engine/EditorBlueprintResources/StandardMacros.FlipFlop` :!label _label
        (:`A`
          (bind (_direction _door_track) (`Timeline|Timeline_0` :!label _label_2)
            (:`Update`
              (`SceneComponent.K2_SetRelativeRotation` (`self.Fdoor`) (`KismetMathLibrary.MakeRotator` 0.0 0.0 (`KismetMathLibrary.Lerp` 0.0 -90.0 _door_track)) false false)
              (set `self.IsDoorClose` false))))
        (:`B`
          (goto _label_2 :!via `Reverse`)))
      (elif (`self.IsEggGone`)
        (set `self.IsDoorClose` true)
        (goto _label)
        (else
          (bind _asbp_first_person_character_2 (cast `/Game/FirstPerson/Blueprints/BP_FirstPersonCharacter` (`GameplayStatics.GetPlayerCharacter` 0)))
          (bind _firstpersonmesh (`/Game/FirstPerson/Blueprints/BP_FirstPersonCharacter.FirstPersonMesh` _asbp_first_person_character_2))
          (bind _returnvalue (`|SpawnActorFromClass` "/Game/Newstuff/KitchenAssets/Egg/BP_egg.BP_egg_C" (`SceneComponent.GetSocketTransform` _firstpersonmesh "GripPoint" "RTS_World") "Undefined" "OverrideRootScale" null null))
          (`self.K2_AttachToComponent` _returnvalue _firstpersonmesh "GripPoint" "SnapToTarget" "SnapToTarget" "SnapToTarget" true)
          (`SceneComponent.SetHiddenInGame` (`self.Egg`) true false)
          (set `self.IsEggGone` true)
          (`GameplayStatics.PlaySound2D` "/Game/Newstuff/KitchenAssets/Voice_Instruction/Crack_The_Egg.Crack_The_Egg" 1.0 1.0 0.0 null null)
          (`PrimitiveComponent.SetRenderCustomDepth` (`self.refrigeratorbody`) false)
          (`PrimitiveComponent.SetRenderCustomDepth` (`self.Fdoor`) false)
          (bind _outactors (`GameplayStatics.GetAllActorsOfClass` "/Game/Newstuff/KitchenAssets/Pan/BP_NewPan.BP_NewPan_C"))
          (`/Engine/EditorBlueprintResources/StandardMacros.CompareInt` (`KismetArrayLibrary.Array_Length` _outactors)
            (:`>`
              (for _array_element _outactors
                _)
              (`PrimitiveComponent.SetRenderCustomDepth` (`/Game/Newstuff/KitchenAssets/Pan/BP_NewPan.pan` _array_element) true))))))))

(event `self.ReceiveTick`
  (params (DeltaSeconds :type "Float (single-precision)"))
  (if (`self.Cat Chaos`)
    (bind _output_get (set `self.counter` (+ 1 (`self.counter`))))
    (`/Engine/EditorBlueprintResources/StandardMacros.CompareInt` _output_get 55
      (:`>`
        (`self.SetActorScale3D` (`self.CatOriginalSize`)))
      (:`<`
        (`self.SetActorScale3D` (- (`self.GetActorScale3D`) (`KismetMathLibrary.MakeVector` 0.0 0.0 (`KismetMathLibrary.RandomFloatInRange` -0.22 0.01))))))))

(fn `UserConstructionScript`)