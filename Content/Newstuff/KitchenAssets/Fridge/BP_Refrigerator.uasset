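; BP_Refrigerator is an interactable kitchen fridge that dispenses eggs.
; Overlap with the UIE component shows its Widget, and end overlap hides it, with no filter on the overlapping actor.
; Interact casts the 1stpov reference to BP_FirstPersonCharacter and spawns a BP_egg at the Target's world transform, printing a message if the cast fails.
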(event `self.UI 'E'.OnComponentBeginOverlap`
  (params (OverlappedComponent :type "PrimitiveComponent Object Reference") (OtherActor :type "Actor Object Reference") (OtherComp :type "PrimitiveComponent Object Reference") (OtherBodyIndex :type Integer) (bFromSweep :type Boolean) (SweepResult :type "HitResult Structure (by ref)"))
  (`SceneComponent.SetHiddenInGame` (`self.Widget`) false false))

(event `self.UI 'E'.OnComponentEndOverlap`
  (params (OverlappedComponent :type "PrimitiveComponent Object Reference") (OtherActor :type "Actor Object Reference") (OtherComp :type "PrimitiveComponent Object Reference") (OtherBodyIndex :type Integer))
  (`SceneComponent.SetHiddenInGame` (`self.Widget`) true false))

(event `/Game/FirstPerson/Blueprints/InteractInterface.Interact`
  (cast `/Game/FirstPerson/Blueprints/BP_FirstPersonCharacter` (`self.1stpov`)
    (:`then`
      (`|SpawnActorFromClass` "/Game/Newstuff/KitchenAssets/Egg/BP_egg.BP_egg_C" (`SceneComponent.K2_GetComponentToWorld` (`self.Target`)) "Undefined" "OverrideRootScale" null null))
    (:`CastFailed`
      (`KismetSystemLibrary.PrintString` "Casting fail"))))

(fn `UserConstructionScript`)