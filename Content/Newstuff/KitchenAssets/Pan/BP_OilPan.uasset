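; BP_OilPan is an oil pan that fills visually as the player interacts using the held oil bottle.
; Box overlap toggles a widget and, the first time, plays a sound and advances the first-person character's objective if it matches.
; HeldOilInteract counts interactions while the bottle overlaps the box, first widening the Oil component, then raising it slightly until a cap is reached.
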(event `self.Box.OnComponentBeginOverlap`
  (params (OverlappedComponent :type "PrimitiveComponent Object Reference") (OtherActor :type "Actor Object Reference") (OtherComp :type "PrimitiveComponent Object Reference") (OtherBodyIndex :type Integer) (bFromSweep :type Boolean) (SweepResult :type "HitResult Structure (by ref)"))
  (`SceneComponent.SetHiddenInGame` (`self.Widget`) false false)
  (`/Engine/EditorBlueprintResources/StandardMacros.DoOnce` false
    (:`Completed`
      (`GameplayStatics.PlaySound2D` "/Game/Newstuff/KitchenAssets/Voice_Instruction/Fridge.Fridge" 1.0 1.0 0.0 null null)
      (bind _asbp_first_person_character (cast `/Game/FirstPerson/Blueprints/BP_FirstPersonCharacter` (`GameplayStatics.GetPlayerCharacter` 0)))
      (if (`KismetStringLibrary.EqualEqual_StrStr` (`/Game/FirstPerson/Blueprints/BP_FirstPersonCharacter.CurrentObjective` _asbp_first_person_character) (`self.Objective`))
        (set `/Game/FirstPerson/Blueprints/BP_FirstPersonCharacter.CurrentObjective` "Put the oil bottle on the shelf next to the oven." _asbp_first_person_character)
        (`/Game/FirstPerson/Blueprints/BP_FirstPersonCharacter.Slide On` _asbp_first_person_character)))))

(event `self.Box.OnComponentEndOverlap`
  (params (OverlappedComponent :type "PrimitiveComponent Object Reference") (OtherActor :type "Actor Object Reference") (OtherComp :type "PrimitiveComponent Object Reference") (OtherBodyIndex :type Integer))
  (`SceneComponent.SetHiddenInGame` (`self.Widget`) true false))

(event `HeldOilInteract`
  (bind _oil (`self.oil`))
  ;[1 1 1] Oil Interact
  (bind _returnvalue (`GameplayStatics.GetActorOfClass` "/Game/Newstuff/KitchenAssets/Oil/BP_HeldOilBottle.BP_HeldOilBottle_C"))
  (if (`PrimitiveComponent.IsOverlappingActor` (`self.Box`) _returnvalue)
    (bind _output_get (set `self.counter` (+ (`self.counter`) 1)))
    (`/Engine/EditorBlueprintResources/StandardMacros.CompareInt` _output_get
      (:`>`
        _)
      (:`==`
        _))
    (`/Engine/EditorBlueprintResources/StandardMacros.CompareInt` _output_get 3
      (:`>`
        (`/Engine/EditorBlueprintResources/StandardMacros.CompareInt` _output_get 5 :!label _label
          (:`<`
            (`SceneComponent.K2_SetWorldLocation` _oil (+ (`SceneComponent.K2_GetComponentLocation` (`self.oil`)) (0.0 0.0 1.0)) false false)
            (`KismetSystemLibrary.PrintString` (`KismetStringLibrary.Conv_IntToString` (`self.counter`))))))
      (:`==`
        (goto _label))
      (:`<`
        (`SceneComponent.SetWorldScale3D` _oil (+ (0.24 0.24 0.0) (`SceneComponent.RelativeScale3D` (`self.oil`))))))))

(fn `UserConstructionScript`)