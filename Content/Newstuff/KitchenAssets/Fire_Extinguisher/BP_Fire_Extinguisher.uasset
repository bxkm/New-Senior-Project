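; Kitchen fire extinguisher actor that the player picks up and carries in the first-person hands.
; Overlapping its box shows a prompt widget, hidden again on exit.
; Interact, once only, spawns a fresh copy attached to the character mesh's GripPoint socket and destroys the original.
; Left mouse press spawns the P_Fire particle emitter attached to the capsule, with no extinguishing logic here.
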(event `self.Box.OnComponentBeginOverlap`
  (params (OverlappedComponent :type "PrimitiveComponent Object Reference") (OtherActor :type "Actor Object Reference") (OtherComp :type "PrimitiveComponent Object Reference") (OtherBodyIndex :type Integer) (bFromSweep :type Boolean) (SweepResult :type "HitResult Structure (by ref)"))
  (`SceneComponent.SetHiddenInGame` (`self.Widget`) false false))

(event `self.Box.OnComponentEndOverlap`
  (params (OverlappedComponent :type "PrimitiveComponent Object Reference") (OtherActor :type "Actor Object Reference") (OtherComp :type "PrimitiveComponent Object Reference") (OtherBodyIndex :type Integer))
  (`SceneComponent.SetHiddenInGame` (`self.Widget`) true false))

(event `/Game/FirstPerson/Blueprints/InteractInterface.Interact`
  ;[1 1 1] Spawn Fire Extinguisher
  (`/Engine/EditorBlueprintResources/StandardMacros.DoOnce` false
    (:`Completed`
      (bind _asbp_first_person_character (cast `/Game/FirstPerson/Blueprints/BP_FirstPersonCharacter` (`GameplayStatics.GetPlayerCharacter` 0))
        (:`then`
          (bind _firstpersonmesh (`/Game/FirstPerson/Blueprints/BP_FirstPersonCharacter.FirstPersonMesh` _asbp_first_person_character))
          (bind _returnvalue (`|SpawnActorFromClass` "BP_Fire_Extinguisher_C" (`SceneComponent.GetSocketTransform` _firstpersonmesh "GripPoint" "RTS_World") "Undefined" "OverrideRootScale" null null))
          (`self.K2_AttachToComponent` _returnvalue _firstpersonmesh "GripPoint" "SnapToTarget" "SnapToTarget" "SnapToTarget" true)
          (`GameplayStatics.GetAllActorsOfClass` "BP_Fire_Extinguisher_C")
          (`self.K2_DestroyActor`))
        (:`CastFailed`
          (`KismetSystemLibrary.PrintString` "no work"))))))

(event `Key|LeftMouseButton`
  (params (Key :type "Key Structure"))
  (bind _capsule (`self.Capsule`))
  (:`Pressed`
    (`GameplayStatics.SpawnEmitterAttached` "/Game/StarterContent/Particles/P_Fire.P_Fire" _capsule "GripPoint" (`SceneComponent.K2_GetComponentLocation` _capsule) (struct) (1.0 1.0 1.0) "KeepWorldPosition")))

(fn `UserConstructionScript`)