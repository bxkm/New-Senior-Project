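; BP_OilShelf is a kitchen shelf where the player puts away the oil bottle as one step of an objective-driven cooking sequence.
; Its box overlap shows a widget while the player character holds oil and hides it on exit.
; ShelfInteract, once the oil pan has spawned, snaps the held bottle to the shelf socket and flags it shelved.
; It then updates the character's objective to the egg step and enables custom-depth rendering on fridges.
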(event `self.Box.OnComponentBeginOverlap`
  (params (OverlappedComponent :type "PrimitiveComponent Object Reference") (OtherActor :type "Actor Object Reference") (OtherComp :type "PrimitiveComponent Object Reference") (OtherBodyIndex :type Integer) (bFromSweep :type Boolean) (SweepResult :type "HitResult Structure (by ref)"))
  (bind _returnvalue (`GameplayStatics.GetActorOfClass` "/Game/FirstPerson/Blueprints/BP_FirstPersonCharacter.BP_FirstPersonCharacter_C"))
  (if (`/Game/FirstPerson/Blueprints/BP_FirstPersonCharacter.HoldingOil` _returnvalue)
    (`SceneComponent.SetHiddenInGame` (`self.Widget`) false false)))

(event `self.Box.OnComponentEndOverlap`
  (params (OverlappedComponent :type "PrimitiveComponent Object Reference") (OtherActor :type "Actor Object Reference") (OtherComp :type "PrimitiveComponent Object Reference") (OtherBodyIndex :type Integer))
  (`SceneComponent.SetHiddenInGame` (`self.Widget`) true false))

(event `ShelfInteract`
  (bind _returnvalue (`GameplayStatics.GetActorOfClass` "/Game/FirstPerson/Blueprints/BP_FirstPersonCharacter.BP_FirstPersonCharacter_C"))
  (if (`/Game/FirstPerson/Blueprints/BP_FirstPersonCharacter.OilPanSpawned` _returnvalue)
    (bind _outactors (`GameplayStatics.GetAllActorsOfClass` "/Game/Newstuff/KitchenAssets/Oil/BP_HeldOilBottle.BP_HeldOilBottle_C"))
    (`/Engine/EditorBlueprintResources/StandardMacros.CompareInt` (`KismetArrayLibrary.Array_Length` _outactors)
      (:`>`
        (`GameplayStatics.GetActorOfClass` "BP_OilShelf_C")
        (bind _returnvalue_2 (`GameplayStatics.GetActorOfClass` "/Game/Newstuff/KitchenAssets/Oil/BP_HeldOilBottle.BP_HeldOilBottle_C"))
        (`self.K2_AttachToComponent` _returnvalue_2 (`self.Actual_Shelves_shelf_2`) "Socket" "SnapToTarget" "SnapToTarget" "SnapToTarget" true)
        (set `self.OilShelved` true)
        (bind _returnvalue_3 (`GameplayStatics.GetActorOfClass` "/Game/FirstPerson/Blueprints/BP_FirstPersonCharacter.BP_FirstPersonCharacter_C"))
        (set `/Game/FirstPerson/Blueprints/BP_FirstPersonCharacter.CurrentObjective` "Get and crack the egg from the fridge into the pan." _returnvalue_3)
        (`/Game/FirstPerson/Blueprints/BP_FirstPersonCharacter.Slide On` _returnvalue_3)
        (bind _outactors_2 (`GameplayStatics.GetAllActorsOfClass` "/Game/Newstuff/KitchenAssets/Fridge/BP_NewFridge.BP_NewFridge_C"))
        (`/Engine/EditorBlueprintResources/StandardMacros.CompareInt` (`KismetArrayLibrary.Array_Length` _outactors_2)
          (:`>`
            (for _array_element _outactors_2
              (`PrimitiveComponent.SetRenderCustomDepth` (`/Game/Newstuff/KitchenAssets/Fridge/BP_NewFridge.refrigeratorbody` _array_element) true)
              (`PrimitiveComponent.SetRenderCustomDepth` (`/Game/Newstuff/KitchenAssets/Fridge/BP_NewFridge.Fdoor` _array_element) true))))))))

(fn `UserConstructionScript`)